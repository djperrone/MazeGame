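; Arrow shooter actor that fires at the player when they step into its line of sight.
; Every tick it sphere-traces a short distance forward from ArrowSource and calls ShootArrow when the player character is hit.
; ShootArrow spawns an Arrow_BP with a sound, using a DoOnce reset after a delay as a cooldown.
; The Box overlap range logic and looping timer are unfinished or disconnected leftovers.
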(event `self.ReceiveBeginPlay`)

(event `ShootArrow`
  (`/Engine/EditorBlueprintResources/StandardMacros.DoOnce` false :!label _label
    (:`Completed`
      (`|SpawnActorFromClass` "/Game/Blueprints/Arrow_BP.Arrow_BP_C" (`SceneComponent.K2_GetComponentToWorld` (`self.ArrowSource`)) "Undefined" "OverrideRootScale" null null)
      (`GameplayStatics.PlaySoundAtLocation` "/Game/Sounds/Arrow_SFX.Arrow_SFX" (`self.K2_GetActorLocation`) (struct) 1.0 1.0 0.0 null null null)
      (`KismetSystemLibrary.Delay` 2.0)
      (goto _label :!via `Reset`))))

(event `self.ReceiveTick`
  (params (DeltaSeconds :type "Float (single-precision)"))
  (bind _arrowsource (`self.ArrowSource`))
  (bind _returnvalue (`SceneComponent.K2_GetComponentLocation` _arrowsource))
  (bind _outhit (`KismetSystemLibrary.SphereTraceSingle` _returnvalue (+ _returnvalue (* (`KismetMathLibrary.GetForwardVector` (`SceneComponent.K2_GetComponentRotation` _arrowsource)) 500)) 10.0 "TraceTypeQuery2"))
  (if (== (`.HitActor` (`GameplayStatics.BreakHitResult` _outhit)) (`GameplayStatics.GetPlayerCharacter` 0))
    (`self.ShootArrow`)))

(event `self.Box.OnComponentBeginOverlap`
  (params (OverlappedComponent :type "PrimitiveComponent Object Reference") (OtherActor :type "Actor Object Reference") (OtherComp :type "PrimitiveComponent Object Reference") (OtherBodyIndex :type Integer) (bFromSweep :type Boolean) (SweepResult :type "HitResult Structure (by ref)"))
  (if (== OtherActor (`GameplayStatics.GetPlayerCharacter` 0))
    _))

(event `self.Box.OnComponentEndOverlap`
  (params (OverlappedComponent :type "PrimitiveComponent Object Reference") (OtherActor :type "Actor Object Reference") (OtherComp :type "PrimitiveComponent Object Reference") (OtherBodyIndex :type Integer))
  (if (== OtherActor (`GameplayStatics.GetPlayerCharacter` 0))
    (set `self.InRange` (`self.False`))))

(fn `UserConstructionScript`)