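; Arrow projectile that damages and knocks back the player on contact.
; When its sphere overlaps a living player, it launches them along the arrow's velocity plus an upward boost, applies damage, destroys itself and plays a hit sound at player 0's location.
; Overlapping any other actor starts a short delay, after which the mesh switches to gravity-driven physics, then the arrow is destroyed after a further delay.
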(event `self.Sphere.OnComponentBeginOverlap`
  (params (OverlappedComponent :type "PrimitiveComponent Object Reference") (OtherActor :type "Actor Object Reference") (OtherComp :type "PrimitiveComponent Object Reference") (OtherBodyIndex :type Integer) (bFromSweep :type Boolean) (SweepResult :type "HitResult Structure (by ref)"))
  (bind _asplayer_character (cast `/Game/Player/PlayerCharacter` OtherActor)
    (:`then`
      (if (> (`/Game/Player/PlayerCharacter.Health` _asplayer_character) 0)
        (`Character.LaunchCharacter` _asplayer_character (+ (`self.GetVelocity`) (0.0 0.0 200.0)) false false)
        (`GameplayStatics.ApplyDamage` _asplayer_character 1.0)
        (`self.K2_DestroyActor`)
        (`GameplayStatics.PlaySoundAtLocation` "/Game/Sounds/Hit_SFX.Hit_SFX" (`self.K2_GetActorLocation` (`GameplayStatics.GetPlayerCharacter` 0)) (struct) 1.0 1.0 0.0 null null null)))
    (:`CastFailed`
      (`KismetSystemLibrary.Delay` 1.5)
      (`PrimitiveComponent.SetEnableGravity` (`self.Sphere`) true)
      (`PrimitiveComponent.SetEnableGravity` (`self.ArrowMesh`) true)
      (`PrimitiveComponent.SetSimulatePhysics` (`self.ArrowMesh`) true)
      (`PrimitiveComponent.SetSimulatePhysics` (`self.Sphere`) false)
      (`KismetSystemLibrary.Delay` 2.0)
      (`self.K2_DestroyActor`))))

(fn `UserConstructionScript`)