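; Broken wall actor that rotates its static mesh when the player character enters its trigger volume, likely to make the wall fall.
; Begin overlap prints a debug greeting and restarts a timeline whose MoveWall track sets the mesh's relative roll, zeroing pitch and yaw.
; End overlap only prints the Fallen variable, which is never set in these graphs; a SetRelativeLocation node is left unconnected.
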(event `self.TriggerVolume.OnComponentBeginOverlap`
  (params (OverlappedComponent :type "PrimitiveComponent Object Reference") (OtherActor :type "Actor Object Reference") (OtherComp :type "PrimitiveComponent Object Reference") (OtherBodyIndex :type Integer) (bFromSweep :type Boolean) (SweepResult :type "HitResult Structure (by ref)"))
  (if (== OtherActor (`GameplayStatics.GetPlayerCharacter` 0))
    (`KismetSystemLibrary.PrintString` "Hello")
    (bind (_direction _movewall) (`Timeline|Timeline_0` :!via `PlayFromStart`)
      (:`Update`
        (`SceneComponent.K2_SetRelativeRotation` (`self.StaticMesh`) (`KismetMathLibrary.MakeRotator` _movewall) false false)))))

(event `self.TriggerVolume.OnComponentEndOverlap`
  (params (OverlappedComponent :type "PrimitiveComponent Object Reference") (OtherActor :type "Actor Object Reference") (OtherComp :type "PrimitiveComponent Object Reference") (OtherBodyIndex :type Integer))
  (if (== OtherActor (`GameplayStatics.GetPlayerCharacter` 0))
    (`KismetSystemLibrary.PrintString` (`KismetStringLibrary.Conv_BoolToString` (`self.Fallen`)))))

(fn `UserConstructionScript`)